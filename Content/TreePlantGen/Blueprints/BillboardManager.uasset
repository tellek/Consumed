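; Manager that sets up billboards for Tree actors and hands out shared pools of billboard texture holders and CAPTURER actors.
; At BeginPlay it sorts trees by camera distance into no billboard, universal holder or individual texture.
; Temporary capturers initialize those billboards and are destroyed, then trees start their on/off checks and a fixed capturer pool is spawned.
; Free-index arrays track both pools, and detected atmospheric fog is passed to capturers as a bug workaround.
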(event `self.ReceiveBeginPlay`
  (bind _returnvalue (`GameplayStatics.GetPlayerCameraManager` 0))
  (for (_ _array_index) (`self.UniversalHolders_Assets`)
    (`KismetArrayLibrary.Array_Add` (`self.freeHoldersIndexes`) _array_index))
  ;[0.05 0.05 0.05] For bug workaround, it's passed into capturers. More info in 'CAPTURER' BP.
  (bind _outactors (`GameplayStatics.GetAllActorsOfClass` "/Script/Engine.AtmosphericFog"))
  (if (> (`KismetArrayLibrary.Array_Length` _outactors) 0)
    (set `self.detectedAtmosphericFog` (`KismetArrayLibrary.Array_Get` _outactors))
    (set `self.AtmosphericFogIsThere` true))
  (`KismetSystemLibrary.Delay` 0.05) ; It must wait for camera manager to initialize.
  ;[0.02238 0.055 0.004036] Fix error when user doesn't have camera manager.
  (`/Engine/EditorBlueprintResources/StandardMacros.IsValid` _returnvalue
    (:`Is Valid`
      (set `self.cameraLocActor` _returnvalue))
    (:`Is Not Valid`
      (set `self.cameraLocActor` (`Controller.GetViewTarget` (`GameplayStatics.GetPlayerController` 0)))))
  (bind _outactors_2 (`GameplayStatics.GetAllActorsOfClass` "/Game/TreePlantGen/Blueprints/InternalLogic/Tree.Tree_C"))
  (for _array_element _outactors_2
    (bind _returnvalue_2 (`self.GetDistanceTo` (`self.cameraLocActor`) _array_element))
    ;[0.01 0.01 0.01] For every tree check its distance to camera and assign to 'universal' or 'individual' billboard texture holders
    (if (> _returnvalue_2 (`self.Billboard_ON_Distance`))
      (if (< _returnvalue_2 (`self.UniversalBillboardMaxDistance`))
        (`KismetArrayLibrary.Array_Add` (`self.initialTreesWithUnivBB`) _array_element)
        (else
          (`KismetArrayLibrary.Array_Add` (`self.initialTreesWithIndividualBB`) _array_element)))
      (else
        (`KismetArrayLibrary.Array_Add` (`self.initialTreesWithoutBB`) _array_element))))
  ;[0.01 0.01 0.01] Spawn initial capturers
  (for _ (range (`KismetArrayLibrary.Array_Length` (`self.initialTreesWithUnivBB`)))
    (bind _returnvalue_3 (`|SpawnActorFromClass` "/Game/TreePlantGen/Blueprints/InternalLogic/CAPTURER.CAPTURER_C" (`self.GetTransform`) "AlwaysSpawn" "OverrideRootScale"))
    (`KismetArrayLibrary.Array_Add` (`self.InitialCapturers`) _returnvalue_3)
    (bind _output_get (set `/Game/TreePlantGen/Blueprints/InternalLogic/CAPTURER.sceneHasAtmosphericFog` (`self.AtmosphericFogIsThere`) _returnvalue_3))
    (if _output_get
      (set `/Game/TreePlantGen/Blueprints/InternalLogic/CAPTURER.atmosphericFog` (`self.detectedAtmosphericFog`) _returnvalue_3)))
  (`KismetSystemLibrary.Delay` 0.01) ; It must wait before the first capture, because spawned capturers need to initialize.
  ;[0 0 0] Initialize universal-holder billboards
  (for (_array_element_2 _array_index_2) (`self.initialTreesWithUnivBB`)
    (set `/Game/TreePlantGen/Blueprints/InternalLogic/Tree.assignedCapturer` (`KismetArrayLibrary.Array_Get` (`self.InitialCapturers`) _array_index_2) _array_element_2)
    (set `/Game/TreePlantGen/Blueprints/InternalLogic/Tree.assignedCapturerIndex` _array_index_2 _array_element_2)
    (bind (_found _foundholder _indexoffoundholder) (`self.GetFreeHolder`))
    (if _found
      (`/Game/TreePlantGen/Blueprints/InternalLogic/Tree.BB_UniversalTexture_ON/OFF` _array_element_2 true _foundholder _indexoffoundholder)
      (else
        (`KismetSystemLibrary.PrintString` "No free universal billboard holder found! Add more to avoid this." true true (struct :`R` 1.0 :`G` 0.123857 :`A` 1.0) 5.0))))
  ;[0 0 0] Initialize individual-holder billboards
  (for _array_element_3 (`self.initialTreesWithIndividualBB`)
    (`/Engine/EditorBlueprintResources/StandardMacros.IsValid` (`/Game/TreePlantGen/Blueprints/InternalLogic/Tree.IndividualBillboardTexture` _array_element_3)
      (:`Is Valid`
        (bind _returnvalue_4 (`|SpawnActorFromClass` "/Game/TreePlantGen/Blueprints/InternalLogic/CAPTURER.CAPTURER_C" (`self.GetTransform`) "AlwaysSpawn" "OverrideRootScale"))
        (bind _returnvalue_5 (`KismetArrayLibrary.Array_Add` (`self.InitialCapturers`) _returnvalue_4))
        (bind _output_get_2 (set `/Game/TreePlantGen/Blueprints/InternalLogic/CAPTURER.sceneHasAtmosphericFog` (`self.AtmosphericFogIsThere`) _returnvalue_4))
        (if _output_get_2
          (set `/Game/TreePlantGen/Blueprints/InternalLogic/CAPTURER.atmosphericFog` (`self.detectedAtmosphericFog`) _returnvalue_4))
        (set `/Game/TreePlantGen/Blueprints/InternalLogic/Tree.assignedCapturer` _returnvalue_4 _array_element_3)
        (set `/Game/TreePlantGen/Blueprints/InternalLogic/Tree.assignedCapturerIndex` _returnvalue_5 _array_element_3)
        (`/Game/TreePlantGen/Blueprints/InternalLogic/Tree.IndividualBillboard_INIT` _array_element_3))
      (:`Is Not Valid`
        (`KismetSystemLibrary.PrintString` "Tree is beyond the distance of universal billboard texture pool, but doesn't have individual billboard texture assigned - it will appear as a normal tree now. Please assign an individual texture for this tree, just like shown in Blueprints/SavedTrees/MySavedTree1/ folder." true true (struct :`R` 1.0 :`G` 0.504862 :`A` 1.0) 20.0)
        (`KismetArrayLibrary.Array_Add` (`self.currentTreesWithoutBBThatShouldBeIndiv`) _array_element_3))))
  ;[0.01 0.01 0.01] Destroy initial capturers and clear the array
  (`self.K2_DestroyActor` (`self.InitialCapturers`))
  (`KismetArrayLibrary.Array_Clear` (`self.availableCapturersIndexes`))
  (set `self.initializationDone` true)
  (`|ExecutionSequence`
    (:`then_0`
      ;[0.01 0.01 0.01] For all trees, start checking if they should turn ON/OFF their billboards.
      (`/Game/TreePlantGen/Blueprints/InternalLogic/Tree.CheckingIf_ON/OFF_Billboard_ON/OFF` (`self.initialTreesWithIndividualBB`) true)
      (`/Game/TreePlantGen/Blueprints/InternalLogic/Tree.CheckingIf_ON/OFF_Billboard_ON/OFF` (`self.initialTreesWithUnivBB`) true)
      (`/Game/TreePlantGen/Blueprints/InternalLogic/Tree.CheckingIf_ON/OFF_Billboard_ON/OFF` (`self.initialTreesWithoutBB`) true))
    (:`then_1`
      ;[0.01 0.01 0.01] Spawn capturers that will be available to use for trees that need it to capture its billboard at specific time.
      (for _ (range 1 (+ (`self.amountOfCapturers`) 1))
        (bind _returnvalue_6 (`|SpawnActorFromClass` "/Game/TreePlantGen/Blueprints/InternalLogic/CAPTURER.CAPTURER_C" (`self.GetTransform`) "AlwaysSpawn" "OverrideRootScale"))
        (bind _returnvalue_7 (`KismetArrayLibrary.Array_Add` (`self.Capturers`) _returnvalue_6))
        (`KismetArrayLibrary.Array_Add` (`self.availableCapturersIndexes`) _returnvalue_7)
        (bind _output_get_3 (set `/Game/TreePlantGen/Blueprints/InternalLogic/CAPTURER.sceneHasAtmosphericFog` (`self.AtmosphericFogIsThere`) _returnvalue_6))
        (if _output_get_3
          (set `/Game/TreePlantGen/Blueprints/InternalLogic/CAPTURER.atmosphericFog` (`self.detectedAtmosphericFog`) _returnvalue_6))))))

(fn `CheckIfFreeHolderExists`
  (returns (Exist :type Boolean))
  (locals (foundHolder_ :type "TextureRenderTarget2D Object Reference") (indexOfFoundHolder_ :type Integer))
  (return (> (`KismetArrayLibrary.Array_Length` (`self.freeHoldersIndexes`)) 0)))

(fn `FreeUpCapturer`
  (params (capturerIndex :type Integer))
  (`KismetArrayLibrary.Array_AddUnique` (`self.availableCapturersIndexes`) capturerIndex))

(fn `FreeUpHolder`
  (params (indexOfHolder :type Integer))
  (locals (waitingTree :type "/Game/TreePlantGen/Blueprints/InternalLogic/Tree Object Reference"))
  (`KismetArrayLibrary.Array_AddUnique` (`self.freeHoldersIndexes`) indexOfHolder) ; Unique just in case.
  (`KismetArrayLibrary.Array_RemoveItem` (`self.indexesOfTAKENHolders_ForDebug`) indexOfHolder))

(fn `GetFreeCapturer`
  (returns (found :type Boolean) (foundCapturer :type "/Game/TreePlantGen/Blueprints/InternalLogic/CAPTURER Object Reference") (foundCapturerIndex :type Integer))
  (locals (foundIndex :type Integer) (indexOfFoundCapturer_ :type Integer) (foundCapturer_ :type "/Game/TreePlantGen/Blueprints/InternalLogic/CAPTURER Object Reference"))
  (bind _availablecapturersindexes (`self.availableCapturersIndexes`))
  (if (> (`KismetArrayLibrary.Array_Length` _availablecapturersindexes) 0)
    (set `local.indexOfFoundCapturer_` (`KismetArrayLibrary.Array_Get` _availablecapturersindexes))
    (set `local.foundCapturer_` (`KismetArrayLibrary.Array_Get` (`self.Capturers`) (`local.indexOfFoundCapturer_`)))
    (`KismetArrayLibrary.Array_Remove` (`self.availableCapturersIndexes`))
    (return true (`local.foundCapturer_`) (`local.indexOfFoundCapturer_`))
    (else
      (return false null -1))))

(fn `GetFreeHolder`
  (returns (Found :type Boolean) (FoundHolder :type "TextureRenderTarget2D Object Reference") (indexOfFoundHolder :type Integer))
  (locals (foundHolder_ :type "TextureRenderTarget2D Object Reference") (indexOfFoundHolder_ :type Integer))
  (bind _indexesoftakenholders_fordebug (`self.indexesOfTAKENHolders_ForDebug`))
  (bind _freeholdersindexes (`self.freeHoldersIndexes`))
  (if (> (`KismetArrayLibrary.Array_Length` _freeholdersindexes) 0)
    (set `local.indexOfFoundHolder_` (`KismetArrayLibrary.Array_Get` _freeholdersindexes))
    (set `local.foundHolder_` (`KismetArrayLibrary.Array_Get` (`self.UniversalHolders_Assets`) (`local.indexOfFoundHolder_`)))
    (`KismetArrayLibrary.Array_Remove` (`self.freeHoldersIndexes`))
    (if (`KismetArrayLibrary.Array_Contains` _indexesoftakenholders_fordebug (`local.indexOfFoundHolder_`))
      (`KismetSystemLibrary.PrintString` "WARNING! Taken a holder that is already taken!" true true (struct :`R` 1.0 :`G` 0.0976 :`A` 1.0)))
    (`KismetArrayLibrary.Array_Add` _indexesoftakenholders_fordebug (`local.indexOfFoundHolder_`))
    (return true (`local.foundHolder_`) (`local.indexOfFoundHolder_`))
    (else
      (return false null 0))))

(fn `UserConstructionScript`)