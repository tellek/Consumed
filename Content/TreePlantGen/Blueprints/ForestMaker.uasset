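; Forest generator actor that scatters trees and plants over the ground within a square area around itself.
; The construction script picks random points, traces down to the surface and previews them as instanced meshes, storing their transforms.
; Trees use a seeded stream, minimum spacing and a slope check, while plants use unseeded random points.
; On BeginPlay the previews are cleared and randomly chosen tree and plant actors spawn at the stored transforms.
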(event `self.ReceiveBeginPlay`
  (bind _treestospawn (`self.TreesToSpawn`))
  (bind _plantstospawn (`self.PlantsToSpawn`))
  (`InstancedStaticMeshComponent.ClearInstances` (`self.InstancedStaticMesh_TreeVis`))
  (`InstancedStaticMeshComponent.ClearInstances` (`self.InstancedPlantVis`))
  (`|ExecutionSequence`
    (:`then_0`
      (for _array_element (`self.transformsToSpawnTrees`)
        (`|SpawnActorFromClass` (`KismetArrayLibrary.Array_Get` _treestospawn (`KismetMathLibrary.RandomIntegerInRange` 0 (- (`KismetArrayLibrary.Array_Length` _treestospawn) 1))) (`KismetMathLibrary.MakeTransform` (.location _array_element) (`KismetMathLibrary.MakeRotator` (.roll (.rotation _array_element)) (.pitch (.rotation _array_element)) (`KismetMathLibrary.RandomFloatInRange` 0.0 360.0)) (.scale _array_element)) "AlwaysSpawn" "OverrideRootScale")))
    (:`then_1`
      (for _array_element_2 (`self.transformsToSpawnPlants`)
        (`|SpawnActorFromClass` (`KismetArrayLibrary.Array_Get` _plantstospawn (`KismetMathLibrary.RandomIntegerInRange` 0 (- (`KismetArrayLibrary.Array_Length` _plantstospawn) 1))) _array_element_2 "AlwaysSpawn" "OverrideRootScale")))))

(fn `UserConstructionScript`
  (locals (randomLoc :type "Vector Structure" :default (0.0 0.0 0.0)) (tooClose :type Boolean) (randStream :type "RandomStream Structure"))
  (bind (_returnvalue_x _returnvalue_y _returnvalue_z) (`KismetMathLibrary.BreakVector` (`self.K2_GetActorLocation`)))
  (bind (_returnvalue_x_2 _returnvalue_y_2 _returnvalue_z_2) (`KismetMathLibrary.BreakVector` (`self.K2_GetActorLocation`)))
  (bind _transformstospawntrees (`self.transformsToSpawnTrees`))
  (bind _forestsize (`self.forestSize`))
  (bind _randstream (`local.randStream`))
  (bind _forestsize_2 (`self.forestSize`))
  (bind _transformstospawnplants (`self.transformsToSpawnPlants`))
  (bind (_randomloc_x _randomloc_y _randomloc_z) (`KismetMathLibrary.BreakVector` (`local.randomLoc`)))
  (bind _returnvalue (* _forestsize -1.0))
  (bind _returnvalue_2 (* _forestsize_2 -1.0))
  (`KismetMathLibrary.SetRandomStreamSeed` (`local.randStream`) (`self.SEED`))
  (`|ExecutionSequence`
    (:`then_0`
      (`KismetArrayLibrary.Array_Clear` (`self.transformsToSpawnTrees`))
      (`KismetArrayLibrary.Array_Clear` (`self.impactNormals`))
      (`KismetArrayLibrary.Array_Clear` (`self.randomLocations`))
      (set `local.tooClose` false)
      (for _ (range 1 (+ (`self.amountOfTrees`) 1))
        (set `local.randomLoc` (`KismetMathLibrary.MakeVector` (+ _returnvalue_x (`KismetMathLibrary.RandomFloatInRangeFromStream` _returnvalue_2 _forestsize_2 _randstream)) (+ _returnvalue_y (`KismetMathLibrary.RandomFloatInRangeFromStream` _returnvalue_2 _forestsize_2 _randstream)) (+ _returnvalue_z 10000.0)))
        (for _array_element (`self.randomLocations`)
          (if (> (`KismetMathLibrary.VSize` (- (`local.randomLoc`) _array_element)) (`self.minDistanceBetweenTrees`))
            (set `local.tooClose` false)
            (else
              (set `local.tooClose` true)
              (break))))
        (if (not (`local.tooClose`))
          (`KismetArrayLibrary.Array_Add` (`self.randomLocations`) (`local.randomLoc`))))
      (for _array_element_2 (`self.randomLocations`)
        (bind _outhit (`KismetSystemLibrary.LineTraceSingle` (`KismetMathLibrary.MakeVector` (.x _array_element_2) (.y _array_element_2) (.z _array_element_2)) (`KismetMathLibrary.MakeVector` (.x _array_element_2) (.y _array_element_2) (- (.z _array_element_2) 15000.0)) "TraceTypeQuery1"))
        (bind (_bblockinghit _binitialoverlap _time _location _impactpoint _normal _impactnormal) (`GameplayStatics.BreakHitResult` _outhit))
        (if (> (.z _impactnormal) (`self.minSlopeRequired`))
          (bind _returnvalue_3 (`KismetArrayLibrary.Array_Add` _transformstospawntrees (`KismetMathLibrary.Conv_VectorToTransform` _location)))
          (`InstancedStaticMeshComponent.AddInstanceWorldSpace` (`self.InstancedStaticMesh_TreeVis`) (`KismetArrayLibrary.Array_Get` _transformstospawntrees _returnvalue_3))
          (`KismetArrayLibrary.Array_Add` (`self.impactNormals`) (`KismetMathLibrary.MakeVector` (.x _impactnormal) (.y _impactnormal) (.z _impactnormal))))))
    (:`then_1`
      (`KismetArrayLibrary.Array_Clear` (`self.transformsToSpawnPlants`))
      (for _ (range 1 (+ (`self.amountOfPlants`) 1))
        (set `local.randomLoc` (`KismetMathLibrary.MakeVector` (+ _returnvalue_x_2 (`KismetMathLibrary.RandomFloatInRange` _returnvalue _forestsize)) (+ _returnvalue_y_2 (`KismetMathLibrary.RandomFloatInRange` _returnvalue _forestsize)) (+ _returnvalue_z_2 10000.0)))
        (bind (_outhit_2 _returnvalue_4) (`KismetSystemLibrary.LineTraceSingle` (`KismetMathLibrary.MakeVector` _randomloc_x _randomloc_y _randomloc_z) (`KismetMathLibrary.MakeVector` _randomloc_x _randomloc_y (- _randomloc_z 15000.0)) "TraceTypeQuery1"))
        (if _returnvalue_4
          (bind _returnvalue_5 (`KismetArrayLibrary.Array_Add` _transformstospawnplants (`KismetMathLibrary.Conv_VectorToTransform` (`.Location` (`GameplayStatics.BreakHitResult` _outhit_2)))))
          (`InstancedStaticMeshComponent.AddInstanceWorldSpace` (`self.InstancedPlantVis`) (`KismetArrayLibrary.Array_Get` _transformstospawnplants _returnvalue_5)))))))