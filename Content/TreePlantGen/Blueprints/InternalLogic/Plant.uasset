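; Procedural plant actor whose construction script builds a random curved spline stem from spline meshes and scatters instanced leaf types along it.
; LOCK freezes the spline and reuses saved leaf growth times and rolls, so hand-edited child Blueprints persist.
; Overlaps trigger a timeline-driven bend away from the other actor through dynamic stem and leaf material parameters.
; A randomly offset looping timer hides the plant and disables its collision beyond cull distance.
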(event `ReactToImpulse`
  (params (Direction :type "Vector Structure") (Strength :type "Float (double-precision)"))
  (bind _returnvalue (`KismetMathLibrary.Conv_VectorToLinearColor` (`KismetMathLibrary.Normal` (`KismetMathLibrary.GreaterGreater_VectorRotator` Direction (struct :`Yaw` 90.0)))))
  (bind _returnvalue_2 (`KismetMathLibrary.MapRangeClamped` (* Strength (`self.Elasticity`)) 0.0 360.0 0.0 1.0))
  (if (not (`self.animIsPlaying`))
    (set `self.animIsPlaying` true)
    (`|ExecutionSequence`
      (:`then_0`
        (`MaterialInstanceDynamic.SetVectorParameterValue` (`self.dynamicStemMat`) "RotAxis" _returnvalue)
        (`MaterialInstanceDynamic.SetVectorParameterValue` (`self.dynamicLeafMaterials`) "RotAxis" _returnvalue)
        (`MaterialInstanceDynamic.SetScalarParameterValue` (`self.dynamicStemMat`) "ImpulseAngle" _returnvalue_2)
        (`MaterialInstanceDynamic.SetScalarParameterValue` (`self.dynamicLeafMaterials`) "ImpulseAngle" _returnvalue_2))
      (:`then_1`
        (bind (_direction _lerp) (`Timeline|ImpulseReactionTimeline` :!via `PlayFromStart`)
          (:`Update`
            (`MaterialInstanceDynamic.SetScalarParameterValue` (`self.dynamicStemMat`) "Impulse" _lerp)
            (`MaterialInstanceDynamic.SetScalarParameterValue` (`self.dynamicLeafMaterials`) "Impulse" _lerp))
          (:`Finished`
            (set `self.animIsPlaying` false)))))))

(event `self.Collider.OnComponentBeginOverlap`
  (params (OverlappedComponent :type "PrimitiveComponent Object Reference") (OtherActor :type "Actor Object Reference") (OtherComp :type "PrimitiveComponent Object Reference") (OtherBodyIndex :type Integer) (bFromSweep :type Boolean) (SweepResult :type "HitResult Structure (by ref)"))
  ;[0 0 0] React to any collision-enabled actor.
  (if (> (`KismetSystemLibrary.GetGameTimeInSeconds`) 1.0)
    (`self.ReactToImpulse` (`KismetMathLibrary.Conv_RotatorToVector` (`KismetMathLibrary.FindLookAtRotation` (`self.K2_GetActorLocation` OtherActor) (`self.K2_GetActorLocation`))) (* (`self.elasticity`) 33.0))))

(event `self.ReceiveBeginPlay`
  (`KismetSystemLibrary.Delay` 0.2)
  (`self.CheckIfCull`)
  (`self.CheckingIfCull_ON/OFF` true))

(event `CheckIfCull`
  ;[1 1 1] Culling, based on distance.
  (if (< (`self.GetDistanceTo` (`GameplayStatics.GetPlayerCameraManager` 0)) (`self.CullDistance`))
    (if (`self.isHidden`)
      (`self.SetActorHiddenInGame` false)
      (set `self.isHidden` false)
      (`PrimitiveComponent.SetCollisionEnabled` (`self.Collider`) "QueryOnly"))
    (elif (not (`self.isHidden`))
      (`self.SetActorHiddenInGame` true)
      (set `self.isHidden` true)
      (`PrimitiveComponent.SetCollisionEnabled` (`self.Collider`) "NoCollision"))))

(event `CheckingIfCull_ON/OFF`
  (params (`ON/OFF` :type Boolean))
  ;[1 1 1] Culling, based on distance.
  (if `ON/OFF`
    (bind _returnvalue (`KismetSystemLibrary.K2_SetTimerDelegate` (delegate `CheckIfCull`) (`KismetMathLibrary.RandomFloatInRange` 1.0 2.0) true))
    (set `self.timer_CheckIfCull` _returnvalue)
    (else
      (`KismetSystemLibrary.K2_ClearAndInvalidateTimerHandle` (`self.timer_CheckIfCull`)))))

(fn `UserConstructionScript`
  (locals (heightOfThePreviousPoint :type "Float (double-precision)") (i :type Integer) (addingMesh :type "SplineMeshComponent Object Reference") (addingLeafType :type "/Game/TreePlantGen/Blueprints/InternalLogic/PlantLeafs Structure" :default (struct)) (randomizedGrowthTime :type "Float (double-precision)") (growthTimesToSave :type "Array of Float (double-precision)") (leafRoll :type "Float (double-precision)") (RollsToSave :type "Array of Float (double-precision)"))
  (bind _returnvalue (`self.K2_GetActorLocation`))
  (bind _addingmesh (`local.addingMesh`))
  (bind _spline (`self.Spline`))
  (bind _addingmesh_2 (`local.addingMesh`))
  (bind _curviness (`self.curviness`))
  (bind _spline_2 (`self.Spline`))
  (bind _spline_3 (`self.Spline`))
  (bind _startscale (`self.startScale`))
  (bind _endscale (`self.endScale`))
  (bind _plantheight (`self.plantHeight`))
  (bind _addingmesh_3 (`local.addingMesh`))
  (bind ((`Angle-Roll_38_E0C1EA66411F031CD7192A9A2FC6EA2B` _angle_roll) (`Angle-Pitch_41_90068CE5476C481DA39116BE5E3824C7` _angle_pitch)) (break `/Game/TreePlantGen/Blueprints/InternalLogic/PlantLeafs` (`local.addingLeafType`)))
  (bind ((`CustomColor_37_77DD992F41ECD4969F1FA59968135A17` _customcolor) (`Color_32_1532323E49F4B7AD02CD1EB6A160F42E` _color) (`ColorGlow_35_57652D304D2FA1B5B92540A270ABB169` _colorglow)) (break `/Game/TreePlantGen/Blueprints/InternalLogic/PlantLeafs` (`local.addingLeafType`)))
  (bind ((`Scale_23_C4D92F274DD3CFDA76DA88A98D6F0D7C` _scale)) (break `/Game/TreePlantGen/Blueprints/InternalLogic/PlantLeafs` (`local.addingLeafType`)))
  (bind ((`growHeight_8_3C11753A4D72A200C04C6396CD4ADFD5` _growheight) (`growHeightTolerance_14_0BBDEF014E0201145DB3ED8E2886FE6D` _growheighttolerance)) (break `/Game/TreePlantGen/Blueprints/InternalLogic/PlantLeafs` (`local.addingLeafType`)))
  (bind ((`Scale_23_C4D92F274DD3CFDA76DA88A98D6F0D7C` _scale_2)) (break `/Game/TreePlantGen/Blueprints/InternalLogic/PlantLeafs` (`local.addingLeafType`)))
  (bind ((`Angle-Roll_38_E0C1EA66411F031CD7192A9A2FC6EA2B` _angle_roll_2) (`Angle-Pitch_41_90068CE5476C481DA39116BE5E3824C7` _angle_pitch_2)) (break `/Game/TreePlantGen/Blueprints/InternalLogic/PlantLeafs` (`local.addingLeafType`)))
  (bind (_location _tangent) (`SplineComponent.GetLocationAndTangentAtSplinePoint` _spline_3 (`local.i`) "Local"))
  (bind _returnvalue_2 (`SplineComponent.GetDirectionAtTime` (`self.Spline`) (`local.randomizedGrowthTime`) "Local" true))
  (bind _returnvalue_3 (* _startscale 0.7))
  (bind _returnvalue_4 (* (`self.curviness`) 0.2))
  (bind _returnvalue_5 (`KismetMathLibrary.MakeVector2D` _returnvalue_3 _returnvalue_3))
  (bind (_location_2 _tangent_2) (`SplineComponent.GetLocationAndTangentAtSplinePoint` _spline_3 (+ (`local.i`) 1) "Local"))
  (bind _returnvalue_6 (`KismetMathLibrary.RandomFloatInRange` (* _curviness -1.0) _curviness))
  (bind _returnvalue_7 (`KismetMathLibrary.RandomFloatInRange` (* _returnvalue_4 -1.0) _returnvalue_4))
  (bind _returnvalue_8 (`KismetMathLibrary.RandomFloatInRange` (* _scale_2 0.9) _scale_2))
  (bind _returnvalue_9 (`KismetMathLibrary.RandomFloatInRange` (* _scale 0.9) _scale))
  (`|ExecutionSequence`
    (:`then_0`
      (if (`self.LOCK`)
        (set `SplineComponent.bInputSplinePointsToConstructionScript` false (`self.Spline`)) ; Important, to be able to save hand-edited blueprint by 'Create child blueprint class'
        (else
          (`SplineComponent.ClearSplinePoints` (`self.Spline`) false)
          (`SplineComponent.AddSplinePoint` (`self.Spline`) (`KismetMathLibrary.MakeVector` 0.0 0.0 -2.0) "Local" false)
          (for _index (range (+ (`self.curveAmount`) 1))
            (set `local.heightOfThePreviousPoint` (+ (`local.heightOfThePreviousPoint`) (`KismetMathLibrary.RandomFloatInRange` (- _plantheight 20.0) _plantheight)))
            (if (== _index 0)
              (`SplineComponent.AddSplinePoint` (`self.Spline`) (`KismetMathLibrary.MakeVector` _returnvalue_7 _returnvalue_7 (`local.heightOfThePreviousPoint`)) "Local" false)
              (else
                (`SplineComponent.AddSplinePoint` (`self.Spline`) (`KismetMathLibrary.MakeVector` _returnvalue_6 _returnvalue_6 (`local.heightOfThePreviousPoint`)) "Local" false))))
          (`SplineComponent.UpdateSpline` (`self.Spline`)))))
    (:`then_1`
      (bind _returnvalue_10 (`KismetMaterialLibrary.CreateDynamicMaterialInstance` (`self.stemMaterial`)))
      (bind _output_get (set `self.dynamicStemMat` _returnvalue_10))
      (`MaterialInstanceDynamic.SetVectorParameterValue` _output_get "LocOfAlpha_0" (`KismetMathLibrary.Conv_VectorToLinearColor` _returnvalue))
      (`MaterialInstanceDynamic.SetVectorParameterValue` _output_get "LocOfAlpha_1" (`KismetMathLibrary.Conv_VectorToLinearColor` (`KismetMathLibrary.MakeVector` (.x _returnvalue) (.y _returnvalue) (.z (`SplineComponent.GetLocationAtTime` (`self.Spline`) 1.0 "World" true)))))
      (`MaterialInstanceDynamic.SetVectorParameterValue` _output_get "RotPivot" (`KismetMathLibrary.Conv_VectorToLinearColor` (`self.K2_GetActorLocation`)))
      (for _index_2 (range (+ (- (`SplineComponent.GetNumberOfSplinePoints` (`self.Spline`)) 2) 1))
        (set `local.i` _index_2)
        (bind _returnvalue_11 (`AddComponent|NODE_AddSplineMeshComponent-0` :`bManualAttachment` true))
        (bind _output_get_2 (set `local.addingMesh` _returnvalue_11))
        (`PrimitiveComponent.SetMaterial` _output_get_2 0 (`self.dynamicStemMat`))
        (`SceneComponent.K2_AttachToComponent` (`local.addingMesh`) (`self.Spline`) "None" "KeepRelative" "KeepRelative" "KeepRelative" true)
        (`|ExecutionSequence`
          (:`then_0`
            (`SplineMeshComponent.SetStartAndEnd` (`local.addingMesh`) _location _tangent _location_2 _tangent_2 false)
            (if (== (`local.i`) 0)
              (`SplineMeshComponent.SetStartScale` _addingmesh (`KismetMathLibrary.MakeVector2D` _startscale _startscale) false)
              (`SplineMeshComponent.SetEndScale` _addingmesh (`KismetMathLibrary.MakeVector2D` _returnvalue_3 _returnvalue_3) false)
              (elif (== (`local.i`) (- (`SplineComponent.GetNumberOfSplinePoints` (`self.Spline`)) 2))
                (`SplineMeshComponent.SetEndScale` _addingmesh_2 (`KismetMathLibrary.MakeVector2D` _endscale _endscale) false)
                (`SplineMeshComponent.SetStartScale` _addingmesh_2 (`KismetMathLibrary.MakeVector2D` _returnvalue_3 _returnvalue_3) false)
                (else
                  (`SplineMeshComponent.SetStartScale` _addingmesh_3 _returnvalue_5 false)
                  (`SplineMeshComponent.SetEndScale` _addingmesh_3 _returnvalue_5 false)))))
          (:`then_1`
            (`SplineMeshComponent.UpdateMesh` (`local.addingMesh`))))))
    (:`then_2`
      (`KismetArrayLibrary.Array_Clear` (`self.dynamicLeafMaterials`)) ; Important!
      (if (not (`self.LOCK`))
        (`KismetArrayLibrary.Array_Clear` (`self.savedLeafData`)))
      (for (_array_element _array_index) (`self.Leaves`)
        (set `local.addingLeafType` _array_element)
        (`|ExecutionSequence`
          (:`then_0`
            (bind _returnvalue_12 (`AddComponent|NODE_AddInstancedStaticMeshComponent-0`))
            (`StaticMeshComponent.SetStaticMesh` _returnvalue_12 (`.Type_22_DCDAB2E64DE53A7D6308EDAED1A49548` (break `/Game/TreePlantGen/Blueprints/InternalLogic/PlantLeafs` (`local.addingLeafType`))))
            (`SceneComponent.K2_AttachToComponent` _returnvalue_12 (`self.Spline`) "None" "KeepRelative" "KeepRelative" "KeepRelative" false)
            (`|ExecutionSequence`
              (:`then_0`
                (bind _returnvalue_13 (`KismetMaterialLibrary.CreateDynamicMaterialInstance` (`PrimitiveComponent.GetMaterial` _returnvalue_12 0)))
                (bind _returnvalue_14 (`MaterialInstanceDynamic.K2_GetVectorParameterValue` (`self.dynamicStemMat`) "LocOfAlpha_0"))
                (`MaterialInstanceDynamic.SetVectorParameterValue` _returnvalue_13 "LocOfAlpha_0" _returnvalue_14)
                (bind _returnvalue_15 (`MaterialInstanceDynamic.K2_GetVectorParameterValue` (`self.dynamicStemMat`) "LocOfAlpha_1"))
                (`MaterialInstanceDynamic.SetVectorParameterValue` _returnvalue_13 "LocOfAlpha_1" _returnvalue_15)
                (bind _returnvalue_16 (`MaterialInstanceDynamic.K2_GetVectorParameterValue` (`self.dynamicStemMat`) "RotPivot"))
                (`MaterialInstanceDynamic.SetVectorParameterValue` _returnvalue_13 "RotPivot" _returnvalue_16)
                (`KismetArrayLibrary.Array_Add` (`self.dynamicLeafMaterials`) _returnvalue_13))
              (:`then_1`
                (`PrimitiveComponent.SetMaterial` _returnvalue_12 0 _returnvalue_13)
                (if _customcolor
                  (`MaterialInstanceDynamic.SetScalarParameterValue` _returnvalue_13 "Colorize" 1.0)
                  (`MaterialInstanceDynamic.SetVectorParameterValue` _returnvalue_13 "Color" _color)
                  (`MaterialInstanceDynamic.SetScalarParameterValue` _returnvalue_13 "Glow" _colorglow)))))
          (:`then_1`
            (if (`self.LOCK`)
              (for _index_3 (range 1 (+ (`.Amount_27_286B227649EE78228EA38F96D574DFCD` (break `/Game/TreePlantGen/Blueprints/InternalLogic/PlantLeafs` (`local.addingLeafType`))) 1))
                (bind (_leafgrowthtimes _leafrolls) (break `/Game/TreePlantGen/Blueprints/InternalLogic/PlantLeafSavedData` (`KismetArrayLibrary.Array_Get` (`self.savedLeafData`) _array_index)))
                (bind _returnvalue_17 (- _index_3 1))
                (bind _item (`KismetArrayLibrary.Array_Get` _leafgrowthtimes _returnvalue_17))
                (bind _returnvalue_18 (`SplineComponent.GetDirectionAtTime` (`self.Spline`) _item "Local" true))
                (`InstancedStaticMeshComponent.AddInstance` _returnvalue_12 (`KismetMathLibrary.MakeTransform` (select `bool` (`.fixedGrowHeight_11_D6247B514C4275BA2873768A42381559` (break `/Game/TreePlantGen/Blueprints/InternalLogic/PlantLeafs` (`local.addingLeafType`))) :`false` (`SplineComponent.GetLocationAtDistanceAlongSpline` _spline (`KismetMathLibrary.RandomFloatInRange` 10.0 (`SplineComponent.GetSplineLength` _spline)) "Local") :`true` (`SplineComponent.GetLocationAtTime` (`self.Spline`) _item "Local" true)) (`KismetMathLibrary.ComposeRotators` (`KismetMathLibrary.ComposeRotators` (`KismetMathLibrary.MakeRotator` (`KismetMathLibrary.RandomFloatInRange` (* _angle_roll_2 0.9) (* _angle_roll_2 1.1)) (`KismetMathLibrary.RandomFloatInRange` (* _angle_pitch_2 0.9) (* _angle_pitch_2 1.1))) (`KismetMathLibrary.MakeRotFromZ` _returnvalue_18)) (`KismetMathLibrary.RotatorFromAxisAndAngle` _returnvalue_18 (`KismetArrayLibrary.Array_Get` _leafrolls _returnvalue_17))) (`KismetMathLibrary.MakeVector` _returnvalue_8 _returnvalue_8 _returnvalue_8))))
              (else
                (for _ (range 1 (+ (`.Amount_27_286B227649EE78228EA38F96D574DFCD` (break `/Game/TreePlantGen/Blueprints/InternalLogic/PlantLeafs` (`local.addingLeafType`))) 1))
                  (bind _output_get_3 (set `local.randomizedGrowthTime` (`KismetMathLibrary.RandomFloatInRange` (- _growheight _growheighttolerance) (+ _growheight _growheighttolerance))))
                  (bind _output_get_4 (set `local.leafRoll` (`KismetMathLibrary.RandomFloatInRange` 0.0 360.0)))
                  (`InstancedStaticMeshComponent.AddInstance` _returnvalue_12 (`KismetMathLibrary.MakeTransform` (select `bool` (`.fixedGrowHeight_11_D6247B514C4275BA2873768A42381559` (break `/Game/TreePlantGen/Blueprints/InternalLogic/PlantLeafs` (`local.addingLeafType`))) :`false` (`SplineComponent.GetLocationAtDistanceAlongSpline` _spline_2 (`KismetMathLibrary.RandomFloatInRange` 10.0 (`SplineComponent.GetSplineLength` _spline_2)) "Local") :`true` (`SplineComponent.GetLocationAtTime` (`self.Spline`) (`local.randomizedGrowthTime`) "Local" true)) (`KismetMathLibrary.ComposeRotators` (`KismetMathLibrary.ComposeRotators` (`KismetMathLibrary.MakeRotator` (`KismetMathLibrary.RandomFloatInRange` (* _angle_roll 0.9) (* _angle_roll 1.1)) (`KismetMathLibrary.RandomFloatInRange` (* _angle_pitch 0.9) (* _angle_pitch 1.1))) (`KismetMathLibrary.MakeRotFromZ` _returnvalue_2)) (`KismetMathLibrary.RotatorFromAxisAndAngle` _returnvalue_2 (`local.leafRoll`))) (`KismetMathLibrary.MakeVector` _returnvalue_9 _returnvalue_9 _returnvalue_9)))
                  (`KismetArrayLibrary.Array_Add` (`local.growthTimesToSave`) _output_get_3)
                  (`KismetArrayLibrary.Array_Add` (`local.RollsToSave`) _output_get_4))
                (`KismetArrayLibrary.Array_Add` (`self.savedLeafData`) (make `/Game/TreePlantGen/Blueprints/InternalLogic/PlantLeafSavedData` (`local.growthTimesToSave`) (`local.RollsToSave`)))
                (`KismetArrayLibrary.Array_Clear` (`local.growthTimesToSave`))
                (`KismetArrayLibrary.Array_Clear` (`local.RollsToSave`))))))))))