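; Fruit actor for the tree and plant generator, showing a configurable mesh and material set in its construction script.
; Fall detaches it from its parent, enables physics-only collision and applies a randomly scaled impulse so it drops.
; A delayed timer then raises angular damping to settle it and finally switches off physics simulation and collision.
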(event `CountToPhysicsTurnOff`
  (bind _mesh (`self.Mesh`))
  (`KismetSystemLibrary.Delay` 5.0)
  (`PrimitiveComponent.SetAngularDamping` _mesh 7.0)
  (`KismetSystemLibrary.Delay` 2.0)
  (`PrimitiveComponent.SetSimulatePhysics` _mesh false)
  (`PrimitiveComponent.SetCollisionEnabled` _mesh "NoCollision"))

(fn `Fall`
  (params (evImpulse :type "Vector Structure"))
  (bind _mesh (`self.Mesh`))
  (`self.K2_DetachFromActor` "KeepWorld" "KeepWorld" "KeepWorld")
  (`PrimitiveComponent.SetCollisionEnabled` _mesh "PhysicsOnly")
  (`PrimitiveComponent.SetSimulatePhysics` _mesh true)
  (`PrimitiveComponent.AddImpulse` _mesh (* evImpulse (`KismetMathLibrary.RandomFloatInRange` 0.5 1.5)) "None" false)
  (`self.CountToPhysicsTurnOff`))

(fn `UserConstructionScript`
  (bind _mesh (`self.Mesh`))
  (`StaticMeshComponent.SetStaticMesh` _mesh (`self.model`))
  (`PrimitiveComponent.SetMaterial` _mesh 0 (`self.material`)))