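; Test actor for the tree generator's wind logic that bends four branch components according to their angle to a wind direction.
; The construction script yaws the Wind component by a test value, caches forward vectors, then processes each branch.
; A dot product with a cross-product sign check yields a 360-degree angle, whose quadrant blends the branch's right and actor's up vectors, signed, into an axis.
; Each branch rotates around that axis by a test angle.
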(fn `setBranchWindAxis`
  (params (galaz :type "ArrowComponent Object Reference"))
  (locals (Branch :type "ArrowComponent Object Reference") (dot :type "Float (double-precision)") (zwrotGalezi :type "Vector Structure") (angle :type "Float (double-precision)") (axis :type "Vector Structure"))
  (bind _angle (`local.angle`))
  (bind _output_get (set `local.Branch` galaz))
  (set `local.zwrotGalezi` (`SceneComponent.GetForwardVector` _output_get))
  (bind _output_get_2 (set `local.dot` (`KismetMathLibrary.Dot_VectorVector` (`local.zwrotGalezi`) (`self.zwrotWiatru!`))))
  (set `local.angle` (`KismetMathLibrary.DegAcos` _output_get_2))
  (if (> (.z (`KismetMathLibrary.Cross_VectorVector` (`local.zwrotGalezi`) (`self.zwrotWiatru!`))) 0.0)
    (`/Engine/EditorBlueprintResources/StandardMacros.NegateFloat` _angle
      (:`  `
        (set `local.angle` (+ _angle 360.0)))))
  (if (`KismetMathLibrary.InRange_FloatFloat` (`local.angle`) 0.0 90.0)
    (set `local.axis` (`KismetMathLibrary.VLerp` (`SceneComponent.GetRightVector` (`local.Branch`)) (* (`self.GetActorUpVector`) -1) (`KismetMathLibrary.MapRangeClamped` (`local.angle`) 0.0 90.0 0.0 1.0)))
    (`SceneComponent.K2_AddWorldRotation` (`local.Branch`) (`KismetMathLibrary.RotatorFromAxisAndAngle` (`local.axis`) (`self.angleTesttttt`)) false false :!label _label)
    (elif (`KismetMathLibrary.InRange_FloatFloat` (`local.angle`) 90.0 180.0)
      (set `local.axis` (`KismetMathLibrary.VLerp` (* (`self.GetActorUpVector`) -1) (* (`SceneComponent.GetRightVector` (`local.Branch`)) -1) (`KismetMathLibrary.MapRangeClamped` (`local.angle`) 90.0 180.0 0.0 1.0)))
      (goto _label)
      (elif (`KismetMathLibrary.InRange_FloatFloat` (`local.angle`) 180.0 270.0)
        (set `local.axis` (`KismetMathLibrary.VLerp` (* (`SceneComponent.GetRightVector` (`local.Branch`)) -1) (`self.GetActorUpVector`) (`KismetMathLibrary.MapRangeClamped` (`local.angle`) 180.0 270.0 0.0 1.0)))
        (goto _label)
        (elif (`KismetMathLibrary.InRange_FloatFloat` (`local.angle`) 270.0 360.0)
          (set `local.axis` (`KismetMathLibrary.VLerp` (`self.GetActorUpVector`) (`SceneComponent.GetRightVector` (`local.Branch`)) (`KismetMathLibrary.MapRangeClamped` (`local.angle`) 270.0 360.0 0.0 1.0)))
          (goto _label))))))

(fn `UserConstructionScript`
  (locals (zwrotGalezi1 :type "Vector Structure" :default (0.0 0.0 0.0)) (zwrotGalezi2 :type "Vector Structure") (zwrotGalezi3 :type "Vector Structure" :default (0.0 0.0 0.0)) (zwrotGalezi4 :type "Vector Structure" :default (0.0 0.0 0.0)))
  (`SceneComponent.K2_SetWorldRotation` (`self.Wind`) (`KismetMathLibrary.MakeRotator` 0.0 0.0 (`self.windRotTesttttt`)) false false)
  (set `local.zwrotGalezi1` (`SceneComponent.GetForwardVector` (`self.branch1`)))
  (set `local.zwrotGalezi2` (`SceneComponent.GetForwardVector` (`self.branch2`)))
  (set `local.zwrotGalezi3` (`SceneComponent.GetForwardVector` (`self.branch3`)))
  (set `local.zwrotGalezi4` (`SceneComponent.GetForwardVector` (`self.branch4`)))
  (set `self.zwrotWiatru!` (`SceneComponent.GetForwardVector` (`self.Wind`)))
  (`self.setBranchWindAxis` (`self.branch1`))
  (`self.setBranchWindAxis` (`self.branch2`))
  (`self.setBranchWindAxis` (`self.branch3`))
  (`self.setBranchWindAxis` (`self.branch4`)))