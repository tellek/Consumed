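; Broken tree piece actor that falls with physics, later becomes pickable and shakes its branches on impact.
; Construction chains scaled capsule colliders between trunk points; double-sided chop pieces simulate on their own mesh, using capsules for click detection.
; Falling pieces get Z-spin damping, then rising angular damping before physics stops, while velocity-drop polling detects ground hits.
; Small double-sided pieces get an impulse, then ramped damping; all double-sided pieces become pickable after a delay.
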(event `self.ReceiveBeginPlay`
  (bind _pointsforcolliders (`self.PointsForColliders`))
  (bind _doublesidedpiecemesh (`self.doubleSidedPieceMesh`))
  (bind _previousvelocity (`self.previousVelocity`))
  (bind _doublesidedpiecemesh_2 (`self.doubleSidedPieceMesh`))
  (`KismetSystemLibrary.Delay` 0.01) ; Important, to include all colliders attached AFTER spawning, in 'SpawnBrokenTreePart' Tree function.
  (if (`self.doubleSidedChopPiece`)
    (`|ExecutionSequence`
      (:`then_0`
        (if (< (`KismetMathLibrary.VSize` (- (`KismetArrayLibrary.Array_Get` _pointsforcolliders) (`KismetArrayLibrary.Array_Get` _pointsforcolliders (`KismetArrayLibrary.Array_LastIndex` _pointsforcolliders)))) 100.0)
          (`PrimitiveComponent.SetAngularDamping` _doublesidedpiecemesh 1.0)
          (`PrimitiveComponent.AddImpulse` _doublesidedpiecemesh (100.0 100.0 50.0) "None" true)
          (`KismetSystemLibrary.Delay` 1.0)
          (`PrimitiveComponent.SetAngularDamping` _doublesidedpiecemesh_2 2.0)
          (`KismetSystemLibrary.Delay` 1.0)
          (`PrimitiveComponent.SetAngularDamping` _doublesidedpiecemesh_2 5.0)
          (`KismetSystemLibrary.Delay` 1.0)
          (`PrimitiveComponent.SetAngularDamping` _doublesidedpiecemesh_2 50.0)))
      (:`then_1`
        (`KismetSystemLibrary.Delay` (`self.pickableAfterXFromFall`))
        (set `self.alreadyPickable` true)))
    (else
      (`|ExecutionSequence`
        (:`then_0`
          (`PrimitiveComponent.SetAllMassScale` (`self.parentCollider`) (`self.massScale`)))
        (:`then_1`
          (bind _returnvalue (`KismetSystemLibrary.K2_SetTimerDelegate` (delegate `LimitAngularZVelocity`) 0.1 true))
          (`KismetSystemLibrary.Delay` 5.0)
          (`KismetSystemLibrary.K2_ClearAndInvalidateTimerHandle` _returnvalue)
          (`PrimitiveComponent.SetAngularDamping` (`self.parentCollider`) 1.0)
          (`KismetSystemLibrary.Delay` 1.0)
          (`PrimitiveComponent.SetAngularDamping` (`self.parentCollider`) 2.0)
          (`KismetSystemLibrary.Delay` 1.0)
          (`PrimitiveComponent.SetAngularDamping` (`self.parentCollider`) 3.0)
          (`KismetSystemLibrary.Delay` 10.0)
          (`PrimitiveComponent.SetSimulatePhysics` (`self.parentCollider`) false))
        (:`then_2`
          ;[0.01 0.01 0.01] Detect if broken tree part hit a ground (sudden velocity decrease)
          (bind _returnvalue_2 (`PrimitiveComponent.GetPhysicsLinearVelocity` (`self.parentCollider`) "None" :!label _label))
          (bind _returnvalue_3 (`KismetMathLibrary.VSize` _returnvalue_2))
          (bind _returnvalue_4 (`KismetMathLibrary.Abs` (- _returnvalue_3 _previousvelocity)))
          (if (and (< _returnvalue_3 _previousvelocity) (> _returnvalue_4 50.0))
            (`|ExecutionSequence`
              (:`then_0`
                (`KismetSystemLibrary.Delay` (`self.pickableAfterXFromFall`))
                (set `self.alreadyPickable` true))
              (:`then_1`
                (for _array_element (`self.allBrokenBranches`)
                  (`/Game/TreePlantGen/Blueprints/InternalLogic/Branch.ShakeFromFalling` _array_element (`KismetMathLibrary.MapRangeClamped` _returnvalue_4 0.0 500.0 0.1 1.0)))))
            (else
              (set `self.previousVelocity` _returnvalue_3)
              (`KismetSystemLibrary.Delay` 0.05)
              (goto _label))))))))

(event `LimitAngularZVelocity`
  (bind _returnvalue (`PrimitiveComponent.GetPhysicsAngularVelocity` (`self.parentCollider`) "None"))
  (bind (_returnvalue_x _returnvalue_y _returnvalue_z) (`KismetMathLibrary.BreakVector` (* (`KismetMathLibrary.NegateVector` _returnvalue) (`self.Angular-Z-Damping`))))
  (`PrimitiveComponent.SetPhysicsAngularVelocity` (`self.parentCollider`) (`KismetMathLibrary.MakeVector` 0.0 0.0 _returnvalue_z) true "None"))

(fn `CreateColliders`
  (locals (i :type Integer))
  (bind _pointsforcolliders (`self.PointsForColliders`))
  (bind _pointsforcolliders_2 (`self.PointsForColliders`))
  (bind _item (`KismetArrayLibrary.Array_Get` _pointsforcolliders 1))
  (bind _item_2 (`KismetArrayLibrary.Array_Get` _pointsforcolliders))
  (bind _item_3 (`KismetArrayLibrary.Array_Get` _pointsforcolliders_2 (+ (`local.i`) 1)))
  (bind _item_4 (`KismetArrayLibrary.Array_Get` (`self.XYScalesForColliders`) (- (`self.breakPointIndex2`) 1)))
  (bind _item_5 (`KismetArrayLibrary.Array_Get` (`self.XYScalesForColliders`) (+ (`self.breakPointIndex2`) (- (`local.i`) 1))))
  (if (`self.doubleSidedChopPiece`)
    (bind _returnvalue (`AddComponent|NODE_AddCapsuleComponent-2`)) ; Single piece uses its own, better collider - so here just add it without physics, to detect clicks
    (set `self.parentCollider` _returnvalue)
    (`PrimitiveComponent.SetSimulatePhysics` (`self.doubleSidedPieceMesh`) true)
    (else
      (bind _returnvalue_2 (`AddComponent|NODE_AddCapsuleComponent-1`)) ; Starting with 100 height (to scale it later) and 30 radius (approx default 'TrunkPiece' mesh radius)
      (set `self.parentCollider` _returnvalue_2)))
  (set `self.firstCollider_Z_Scale` (/ (`KismetMathLibrary.VSize` (- _item_2 _item)) 200.0))
  (`SceneComponent.K2_SetWorldTransform` (`self.parentCollider`) (`KismetMathLibrary.MakeTransform` (/ (+ _item_2 _item) 2) (`KismetMathLibrary.Conv_VectorToRotator` (`KismetMathLibrary.GetUpVector` (`KismetMathLibrary.FindLookAtRotation` _item_2 _item))) (`KismetMathLibrary.MakeVector` _item_4 _item_4 (`self.firstCollider_Z_Scale`))) false false)
  (if (> (`KismetArrayLibrary.Array_Length` (`self.PointsForColliders`)) 2)
    (for _index (range 1 (+ (- (`KismetArrayLibrary.Array_Length` (`self.PointsForColliders`)) 2) 1))
      (bind _output_get (set `local.i` _index))
      (bind _returnvalue_3 (`AddComponent|NODE_AddCapsuleComponent-0`)) ; Starting with 100 height (to scale it later) and 30 radius (approx default 'TrunkPiece' mesh radius)
      (`SceneComponent.K2_AttachToComponent` _returnvalue_3 (`self.parentCollider`) "None" "KeepRelative" "KeepRelative" "KeepRelative" true)
      (bind _item_6 (`KismetArrayLibrary.Array_Get` _pointsforcolliders_2 _output_get))
      (`SceneComponent.K2_SetWorldTransform` _returnvalue_3 (`KismetMathLibrary.MakeTransform` (/ (+ _item_6 _item_3) 2) (`KismetMathLibrary.Conv_VectorToRotator` (`KismetMathLibrary.GetUpVector` (`KismetMathLibrary.FindLookAtRotation` _item_6 _item_3))) (`KismetMathLibrary.MakeVector` _item_5 _item_5 (/ (`KismetMathLibrary.VSize` (- _item_6 _item_3)) 200.0))) false false))))

(fn `UserConstructionScript`
  (`self.CreateColliders`))