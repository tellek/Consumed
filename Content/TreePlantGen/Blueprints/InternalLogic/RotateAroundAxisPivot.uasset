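; Helper actor in the TreePlantGen internal logic that rotates a point component around a pivot component.
; On construction it reads the world positions of Piwot and Punkt, converts the point into pivot-relative space and rotates it by Degrees around AXIS.
; It then transforms the result back to world space and moves Punkt there.
; The event graph is empty, so all work happens in the Construction Script.
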(fn `UserConstructionScript`
  (set `self.PivotPoint` (`SceneComponent.K2_GetComponentLocation` (`self.piwot`)))
  (set `self.PointToRotate` (`SceneComponent.K2_GetComponentLocation` (`self.punkt`)))
  (`SceneComponent.K2_SetWorldLocation` (`self.punkt`) (`KismetMathLibrary.TransformLocation` (`KismetMathLibrary.Conv_VectorToTransform` (`self.PivotPoint`)) (`KismetMathLibrary.RotateAngleAxis` (`KismetMathLibrary.InverseTransformLocation` (`KismetMathLibrary.Conv_VectorToTransform` (`self.PivotPoint`)) (`self.PointToRotate`)) (`self.Degrees`) (`self.AXIS`))) false false))